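; Dirt tile Blueprint for the board game, filed under the second-generation grassland biome tiles.
; Its one working function, ChangeDecalColor, sets the DecalTint parameter on the DynamicDecal material.
; Events and the construction script are empty; hover highlight, grid-number debug text and dynamic decal creation are disconnected, so this graph never assigns DynamicDecal.
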(event MouseInput|EventActorBeginCursorOver)

(event Collision|EventActorBeginOverlap
  (params (OtherActor :type Actor%20Object%20Reference)))

(event EventBeginPlay)

(fn ConstructionScript)

(fn ChangeDecalColor
  (params (Color :type Color%20Structure))
  (Rendering|Material|SetVectorParameterValue (Variables|Default|GetdynamicDecal) "DecalTint" (Math|Conversions|ToLinearColor(Color) Color) :!class /Script/Engine.MaterialInstanceDynamic))