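; Animated fish actor for the board game, a child Blueprint that inherits its behavior from a parent class.
; Its playAnimation override calls the parent version with SkeletalMesh and AnimationAsset, leaving playback to the parent.
; The construction script only calls its parent, and the BeginPlay, overlap and Tick events are disabled placeholders.
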(event EventBeginPlay
  (|CallParentFunction) ; This node is disabled and will not be called.\nDrag off pins to build functionality.
)

(event Collision|EventActorBeginOverlap
  (params (OtherActor :type Actor%20Object%20Reference))
  (|CallParentFunction OtherActor) ; This node is disabled and will not be called.\nDrag off pins to build functionality.
)

(event EventTick
  (params (DeltaSeconds :type Float%20%28single-precision%29))
  (|CallParentFunction DeltaSeconds) ; This node is disabled and will not be called.\nDrag off pins to build functionality.
)

(fn ConstructionScript
  (|CallParentFunction))

(fn PlayAnimation
  (params (skeletal%20mesh :type Skeletal%20Mesh%20Component%20Object%20Reference) (animation%20to%20play :type Animation%20Asset%20Object%20Reference))
  (|CallParentFunction (Variables|Default|GetSkeletalMesh) (Variables|Default|Getanimation%20asset)))